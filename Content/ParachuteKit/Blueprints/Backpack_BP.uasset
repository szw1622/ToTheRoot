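; Parachute kit backpack Blueprint that lets the backpack mesh switch between five skins: camo, fabric, RWB, skull and target.
; ChangeTexture_B passes an index through an authority check to a server event, so only the authority path triggers the change.
; That event calls ChangeTextureF, which maps the index to a material and applies it to the first slot of BackpackMesh.
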(event `ChangeTexture_B`
  (params (StartNumber :type Integer))
  ;[1 1 1] Change Texture
  (`/Engine/EditorBlueprintResources/ActorMacros.Switch Has Authority`
    (:`Authority`
      (`self.ChangeTexture_B_Server` StartNumber))))

(event `ChangeTexture_B_Server`
  (params (StartNumber :type Integer))
  ;[1 1 1] Change Texture
  (`self.ChangeTextureF` StartNumber))

(fn `ChangeTextureF`
  (params (StartNumber :type Integer))
  ;[1 1 1] Set New Texture
  (switch `int` StartNumber
    (:`0`
      (set `self.NewTexture` "/Game/ParachuteKit/Materials/Backpack/BSK_Camo_M.BSK_Camo_M"))
    (:`1`
      (set `self.NewTexture` "/Game/ParachuteKit/Materials/Backpack/BSK_Fabric_M.BSK_Fabric_M"))
    (:`2`
      (set `self.NewTexture` "/Game/ParachuteKit/Materials/Backpack/BSK_RWB_M.BSK_RWB_M"))
    (:`3`
      (set `self.NewTexture` "/Game/ParachuteKit/Materials/Backpack/BSK_Skull_M.BSK_Skull_M"))
    (:`4`
      (set `self.NewTexture` "/Game/ParachuteKit/Materials/Backpack/BSK_Target_M.BSK_Target_M")))
  ;[1 1 1] Apply New Texture
  (`PrimitiveComponent.SetMaterial` (`self.BackpackMesh`) 0 (`self.NewTexture`)))

(fn `UserConstructionScript`)