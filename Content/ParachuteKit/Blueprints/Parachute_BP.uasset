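; Parachute actor that shows deploy, open-idle and landing animations on its mesh and can switch between five canopy materials.
; Each public event passes an authority check, then forwards to a matching Server event that does the work directly or through helper functions.
; Deploy makes the mesh visible, plays once, then switches to the looping open animation after a fixed delay.
; The standalone idle event waits the same delay before looping.
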(event `ChangeTexture_P`
  (params (`Start Number` :type Integer))
  ;[1 1 1] Change texture
  (`/Engine/EditorBlueprintResources/ActorMacros.Switch Has Authority`
    (:`Authority`
      (`self.ChangeTexture_P_Server` `Start Number`))))

(event `ChangeTexture_P_Server`
  (params (`Start Number` :type Integer))
  ;[1 1 1] Change texture
  (`self.ChangeTextureF` `Start Number`))

(event `ParachuteLandAnim`
  ;[1 1 1] Parachute Land Animation
  (`/Engine/EditorBlueprintResources/ActorMacros.Switch Has Authority`
    (:`Authority`
      (`self.ParachuteLandAnim_Server`))))

(event `ParachuteLandAnim_Server`
  ;[1 1 1] Parachute Land Animation
  (`SkeletalMeshComponent.PlayAnimation` (`self.ParachuteMesh`) "/Game/ParachuteKit/Animations/Parachute/P_ParachuteLand.P_ParachuteLand" false))

(event `ParachuteDeployAnim`
  ;[1 1 1] Deploy Parachute
  (`/Engine/EditorBlueprintResources/ActorMacros.Switch Has Authority`
    (:`Authority`
      (`self.ParachuteDeployAnim_Server`))))

(event `ParachuteDeployAnim_Server`
  ;[1 1 1] Deploy Parachute
  (`self.ParachuteDeployF`)
  (`KismetSystemLibrary.Delay` 1.958)
  (`self.ParachuteIdleF`))

(event `ParachuteIdleAnim`
  ;[1 1 1] Parachute Idle
  (`/Engine/EditorBlueprintResources/ActorMacros.Switch Has Authority`
    (:`Authority`
      (`self.ParachuteIdleAnim_Server`))))

(event `ParachuteIdleAnim_Server`
  ;[1 1 1] Parachute Idle
  (`KismetSystemLibrary.Delay` 1.958)
  (`self.ParachuteIdleF`))

(fn `ChangeTextureF`
  (params (StartNumber :type Integer))
  ;[1 1 1] Set New Texture
  (switch `int` StartNumber
    (:`0`
      (set `self.NewTexture` "/Game/ParachuteKit/Materials/Parachute/P_Camo_M.P_Camo_M"))
    (:`1`
      (set `self.NewTexture` "/Game/ParachuteKit/Materials/Parachute/P_Fabric_M.P_Fabric_M"))
    (:`2`
      (set `self.NewTexture` "/Game/ParachuteKit/Materials/Parachute/P_RWB_M.P_RWB_M"))
    (:`3`
      (set `self.NewTexture` "/Game/ParachuteKit/Materials/Parachute/P_Skull_M.P_Skull_M"))
    (:`4`
      (set `self.NewTexture` "/Game/ParachuteKit/Materials/Parachute/P_Target_M.P_Target_M")))
  ;[1 1 1] Apply New Texture
  (`PrimitiveComponent.SetMaterial` (`self.ParachuteMesh`) 0 (`self.NewTexture`)))

(fn `ParachuteDeployF`
  ;[1 1 1] Set Visible
  (`SceneComponent.SetVisibility` (`self.ParachuteMesh`) true false)
  ;[1 1 1] Play Deploy Animation Once
  (`SkeletalMeshComponent.PlayAnimation` (`self.ParachuteMesh`) "/Game/ParachuteKit/Animations/Parachute/P_ParachuteDeploy.P_ParachuteDeploy" false))

(fn `ParachuteIdleF`
  ;[1 1 1] Play Idle Animation (Loop)
  (`SkeletalMeshComponent.PlayAnimation` (`self.ParachuteMesh`) "/Game/ParachuteKit/Animations/Parachute/P_ParachuteOpen.P_ParachuteOpen" true))

(fn `UserConstructionScript`)